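; Plant pot actor that takes dirt and a seed, feeds the spawned StarterPlant_BP, and handles harvest.
; Planting copies seed requirements to the plant and nutrient widget, then starts one-second recursive Delay loops draining health and nutrients.
; Nutrient drain scales with growth stage, except water; levels are pushed to plant and widget, and AddNutrients tops them up.
; Harvest docks quality for growth and pruning faults; the player-facing widget shows on overlap.
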(event `self.ReceiveBeginPlay`
  (bind _asnutrient_w (cast `/Game/Plant/Nutrient_W` (`WidgetComponent.GetUserWidgetObject` (`self.NuteStats`))))
  (set `self.As Nutrient W` _asnutrient_w)
  (`self.SetWidgetValues`)
  (`SceneComponent.SetHiddenInGame` (`self.NuteStats`) true false))

(event `self.ReceiveTick`
  (params (DeltaSeconds :type "Float (single-precision)"))
  (bind _returnvalue (`GameplayStatics.GetPlayerCharacter` 0))
  (bind _nutestats (`self.NuteStats`))
  (`SceneComponent.K2_SetWorldRotation` _nutestats (`KismetMathLibrary.FindLookAtRotation` (`SceneComponent.K2_GetComponentLocation` _nutestats) (+ (`self.K2_GetActorLocation` _returnvalue) (0.0 0.0 60.0))) false false)
  (`SceneComponent.K2_SetWorldRotation` (`self.Spline`) (`KismetMathLibrary.MakeRotator` 0.0 0.0 (+ (.yaw (`KismetMathLibrary.FindLookAtRotation` (`SceneComponent.K2_GetComponentLocation` (`self.Spline`)) (`self.K2_GetActorLocation` _returnvalue))) -120.0)) false false))

(event `OnInteract`
  (if (`self.isPlanted`)
    (`self.PlantSeed` null)
    (else
      (`self.Harvest`))))

(event `PlaceDirt`
  (params (Nitrogen :type "Float (double-precision)") (Phosphorus :type "Float (double-precision)") (Potassium :type "Float (double-precision)") (MicroNutrients :type "Float (double-precision)") (Water :type "Float (double-precision)"))
  (`SceneComponent.SetHiddenInGame` (`self.Dirt`) false false)
  (set `self.isDirted` true)
  (`self.SetPotNutrients` Nitrogen Phosphorus Potassium MicroNutrients Water)
  (`self.SetWidgetValues`))

(event `PlantSeed`
  (params (PlayerHeldActor :type "Actor Object Reference"))
  (bind _as_nutrient_w (`self.As Nutrient W`))
  (if (not (`self.isPlanted`))
    (set `self.isPlanted` true)
    (bind _asseed_m (cast `/Game/Plant/BPs/Seeds/Seed_M` PlayerHeldActor))
    (bind _output_get (set `self.As Seed M` _asseed_m))
    (bind _returnvalue (`|SpawnActorFromClass` "/Game/Plant/BPs/Plants/StarterPlant_BP.StarterPlant_BP_C" (`KismetMathLibrary.MakeTransform` (+ (`self.K2_GetActorLocation`) (0.0 0.0 40.0)) (struct) (0.25 0.25 0.25)) "Undefined" "MultiplyWithRoot" null null))
    (bind _output_get_2 (set `self.PlantInPot` _returnvalue))
    (bind _output_get_3 (set `/Game/Plant/BPs/Plants/Plant_M.BestNitrogen` (`/Game/Plant/BPs/Seeds/Seed_M.BestNitrogen` _output_get) _output_get_2))
    (bind _output_get_4 (set `/Game/Plant/BPs/Plants/Plant_M.BestPhosphorus` (`/Game/Plant/BPs/Seeds/Seed_M.BestPhosphorus` _output_get) _output_get_2))
    (bind _output_get_5 (set `/Game/Plant/BPs/Plants/Plant_M.BestPotassium` (`/Game/Plant/BPs/Seeds/Seed_M.BestPotassium` _output_get) _output_get_2))
    (bind _output_get_6 (set `/Game/Plant/BPs/Plants/Plant_M.BestMicroNutrients` (`/Game/Plant/BPs/Seeds/Seed_M.BestMicroNutrients` _output_get) _output_get_2))
    (bind _output_get_7 (set `/Game/Plant/BPs/Plants/Plant_M.BestWater` (`/Game/Plant/BPs/Seeds/Seed_M.BestWater` _output_get) _output_get_2))
    (set `/Game/Plant/BPs/Plants/Plant_M.TimeUntilPrune` (`/Game/Plant/BPs/Seeds/Seed_M.TimeUntilPrune` _output_get) _output_get_2)
    (set `/Game/Plant/BPs/Plants/Plant_M.BestDryTime` (`/Game/Plant/BPs/Seeds/Seed_M.BestDryTime` _output_get) _output_get_2)
    (set `/Game/Plant/BPs/Plants/Plant_M.requiresPrune` (`/Game/Plant/BPs/Seeds/Seed_M.requiresPrune` _output_get) _output_get_2)
    (`self.SetWidgetValues`)
    (`self.Decay`)
    (`self.NutrientDecay`)
    (set `/Game/Plant/Nutrient_W.BestNitrogen` _output_get_3 _as_nutrient_w)
    (set `/Game/Plant/Nutrient_W.BestPhosphorus` _output_get_4 _as_nutrient_w)
    (set `/Game/Plant/Nutrient_W.BestPotassium` _output_get_5 _as_nutrient_w)
    (set `/Game/Plant/Nutrient_W.BestMicroNutrients` _output_get_6 _as_nutrient_w)
    (set `/Game/Plant/Nutrient_W.BestWater` _output_get_7 _as_nutrient_w)))

(event `Decay`
  (if (`self.isPlanted`)
    (`KismetSystemLibrary.Delay` 1.0)
    (set `self.Health` (- (`self.Health`) (`self.PhyiscalDecay`)))
    (`self.Decay`)))

(event `Harvest`
  (bind (_isplanted _health _phyiscaldecay _plantinpot _nitrogen _phosphorus _potassium _micronutrients _nutedecayconst _water) (defaults `/Game/Plant/BPs/Pots/FirstPot_BP` "FirstPot_BP_C"))
  (bind _plantinpot_2 (`self.PlantInPot`))
  (bind _plantinpot_3 (`self.PlantInPot`))
  (bind _plantinpot_4 (`self.PlantInPot`))
  (bind _growthlevel (`/Game/Plant/BPs/Plants/Plant_M.GrowthLevel` _plantinpot_4))
  (bind _growthtimecount (`/Game/Plant/BPs/Plants/Plant_M.GrowthTimeCount` _plantinpot_4))
  (bind _returnvalue (`KismetMathLibrary.Abs` (- _growthlevel _growthtimecount)))
  (if (`self.isPlanted`)
    (if (or (>= _growthlevel 1500.0) (>= _growthtimecount 1500))
      (set `self.Quality` (- (`self.Quality`) 1.5)))
    (if (> _returnvalue 600.0)
      (set `self.Quality` (- (`self.Quality`) 0.5))
      (if (>= _returnvalue 800.0)
        (set `self.Quality` (- (`self.Quality`) 0.5))
        (if (>= _returnvalue 900.0)
          (set `self.Quality` (- (`self.Quality`) 0.5))
          (if (>= _returnvalue 1000.0)
            (set `self.Quality` (- (`self.Quality`) 0.5))
            (if (>= _returnvalue 1200.0)
              (bind _output_get (set `self.Quality` (- (`self.Quality`) 0.5))))))))
    (if (`/Game/Plant/BPs/Plants/Plant_M.requiresPrune` _plantinpot_2)
      (if (not (`/Game/Plant/BPs/Plants/Plant_M.beenPruned` _plantinpot_2))
        (set `self.Quality` (- (`self.Quality`) 0.5))))
    (set `/Game/Plant/BPs/Plants/Plant_M.isHarvested` true _plantinpot_3)
    (set `/Game/Plant/BPs/Plants/Plant_M.Quality` _output_get _plantinpot_3)
    (`SceneComponent.SetHiddenInGame` (`self.Dirt`) false false)
    (set `self.isDirted` false)
    (set `self.isPlanted` false)
    (`self.SetPotNutrients` _nitrogen _phosphorus _potassium _micronutrients _water)))

(event `NutrientDecay`
  (bind _nutedecaymultiplier (`self.NuteDecayMultiplier`))
  (bind _returnvalue (- (`self.Water`) 0.2))
  (bind _returnvalue_2 (- (`self.MicroNutrients`) (* (`self.NuteDecayConst`) _nutedecaymultiplier)))
  (bind _returnvalue_3 (- (`self.Phosphorus`) (* (`self.NuteDecayConst`) _nutedecaymultiplier)))
  (bind _returnvalue_4 (- (`self.Nitrogen`) (* (`self.NuteDecayConst`) _nutedecaymultiplier)))
  (bind _returnvalue_5 (- (`self.Potassium`) (* (`self.NuteDecayConst`) _nutedecaymultiplier)))
  (`self.SetNuteDecayMulti`)
  (if (`self.isPlanted`)
    (if (not (<= _returnvalue_4 0.0))
      (set `self.Nitrogen` _returnvalue_4))
    (if (not (<= _returnvalue_3 0.0))
      (set `self.Phosphorus` _returnvalue_3))
    (if (not (<= _returnvalue_5 0.0))
      (set `self.Potassium` _returnvalue_5))
    (if (not (<= _returnvalue_2 0.0))
      (set `self.MicroNutrients` _returnvalue_2))
    (if (not (<= _returnvalue 0.0))
      (set `self.Water` _returnvalue))
    ;[1 1 1] Collapsed Function
    (`self.SetPlantNutrients`)
    (`self.SetWidgetValues`)
    (`KismetSystemLibrary.Delay` 1.0)
    (`self.NutrientDecay`)))

(event `AddNutrients`
  (params (Selection :type String) (NutrientAddAmount :type "Float (double-precision)"))
  (bind _output_get (set `self.NutrientAddAmount` NutrientAddAmount))
  (switch `string` Selection
    (:`Nitrogen_BP_C`
      (set `self.Nitrogen` (+ _output_get (`self.Nitrogen`))))
    (:`Phosphorus_BP_C`
      (set `self.Phosphorus` (+ _output_get (`self.Phosphorus`))))
    (:`Potassium_BP_C`
      (set `self.Potassium` (+ _output_get (`self.Potassium`))))
    (:`MicroNutrients_BP_C`
      (set `self.MicroNutrients` (+ _output_get (`self.MicroNutrients`))))
    (:`Water_BP_C`
      (set `self.Water` (+ _output_get (`self.Water`)))))
  (`self.SetWidgetValues`))

(event `self.Capsule.OnComponentBeginOverlap`
  (params (OverlappedComponent :type "PrimitiveComponent Object Reference") (OtherActor :type "Actor Object Reference") (OtherComp :type "PrimitiveComponent Object Reference") (OtherBodyIndex :type Integer) (bFromSweep :type Boolean) (SweepResult :type "HitResult Structure (by ref)"))
  (cast `/Game/FirstPerson/Blueprints/BP_FirstPersonCharacter` OtherActor)
  (`SceneComponent.SetHiddenInGame` (`self.NuteStats`) false false))

(event `self.Capsule.OnComponentEndOverlap`
  (params (OverlappedComponent :type "PrimitiveComponent Object Reference") (OtherActor :type "Actor Object Reference") (OtherComp :type "PrimitiveComponent Object Reference") (OtherBodyIndex :type Integer))
  (cast `/Game/FirstPerson/Blueprints/BP_FirstPersonCharacter` OtherActor)
  (`SceneComponent.SetHiddenInGame` (`self.NuteStats`) true false))

(fn `SetNuteDecayMulti`
  (bind _growthstage (`/Game/Plant/BPs/Plants/Plant_M.GrowthStage` (`self.PlantInPot`)))
  (if (<= _growthstage 0)
    (set `self.NuteDecayMultiplier` 1.0)
    (elif (== _growthstage 1)
      (set `self.NuteDecayMultiplier` 1.2)
      (elif (== _growthstage 2)
        (set `self.NuteDecayMultiplier` 1.4)
        (elif (== _growthstage 3)
          (set `self.NuteDecayMultiplier` 1.6)
          (elif (>= _growthstage 4)
            (set `self.NuteDecayMultiplier` 3.0)))))))

(fn `SetPlantNutrients`
  (bind _plantinpot (`self.PlantInPot`))
  (set `/Game/Plant/BPs/Plants/Plant_M.Nitrogen` (`self.Nitrogen`) _plantinpot)
  (set `/Game/Plant/BPs/Plants/Plant_M.Phosphorus` (`self.Phosphorus`) _plantinpot)
  (set `/Game/Plant/BPs/Plants/Plant_M.Potassium` (`self.Potassium`) _plantinpot)
  (set `/Game/Plant/BPs/Plants/Plant_M.MicroNutrients` (`self.MicroNutrients`) _plantinpot)
  (set `/Game/Plant/BPs/Plants/Plant_M.Water` (`self.Water`) _plantinpot))

(fn `SetPotNutrients`
  (params (Nitrogen :type "Float (double-precision)") (Phosphorus :type "Float (double-precision)") (Potassium :type "Float (double-precision)") (MicroNutrients :type "Float (double-precision)") (Water :type "Float (double-precision)"))
  (set `self.Nitrogen` Nitrogen)
  (set `self.Phosphorus` Phosphorus)
  (set `self.Potassium` Potassium)
  (set `self.MicroNutrients` MicroNutrients)
  (set `self.Water` Water))

(fn `SetWidgetValues`
  (bind _as_nutrient_w (`self.As Nutrient W`))
  (set `/Game/Plant/Nutrient_W.Nitrogen` (`self.Nitrogen`) _as_nutrient_w)
  (set `/Game/Plant/Nutrient_W.Phosphorus` (`self.Phosphorus`) _as_nutrient_w)
  (set `/Game/Plant/Nutrient_W.Potassium` (`self.Potassium`) _as_nutrient_w)
  (set `/Game/Plant/Nutrient_W.MicroNutrients` (`self.MicroNutrients`) _as_nutrient_w)
  (set `/Game/Plant/Nutrient_W.Water` (`self.Water`) _as_nutrient_w))

(fn `UserConstructionScript`
  (`parent.UserConstructionScript`))