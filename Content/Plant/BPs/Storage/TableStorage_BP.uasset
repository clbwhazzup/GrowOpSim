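; Table storage Blueprint that tracks a fixed set of item socket slots and hands out free positions for items.
; On BeginPlay it overlap-checks each socket, flagging it occupied when it finds an actor, but stops checking that socket on a Nutes_M, Seed_M or Dirt_M match.
; Organize picks the first unflagged socket, stores its world position in ItemLocation and flags it occupied.
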(event `self.ReceiveBeginPlay`
  (bind _output_get (set `self.ItemSockets` (`|MakeArray` (`self.ItemSocket0`) (`self.ItemSocket1`) (`self.ItemSocket2`) (`self.ItemSocket3`) (`self.ItemSocket4`) (`self.ItemSocket5`) (`self.ItemSocket6`) (`self.ItemSocket7`) (`self.ItemSocket8`) (`self.ItemSocket9`) (`self.ItemSocket10`))))
  (for (_array_element _array_index) _output_get
    (bind _outactors (`KismetSystemLibrary.ComponentOverlapActors` _array_element (`KismetMathLibrary.MakeTransform` (`SceneComponent.K2_GetComponentLocation` _array_element)) (`|MakeArray` "ObjectTypeQuery2" "ObjectTypeQuery1" :!type "EObjectTypeQuery Enum")))
    (for _array_element_2 _outactors
      (if (or (== _array_element_2 "/Game/Plant/BPs/Nutes/Nutes_M.Nutes_M") (== _array_element_2 "/Game/Plant/BPs/Seeds/Seed_M.Seed_M") (== _array_element_2 "/Game/Plant/BPs/Dirt/Dirt_M.Dirt_M"))
        (break)
        (else
          (`KismetArrayLibrary.Array_Set` (`self.ArrayBool`) _array_index true))))))

(event `Organize`
  (bind _array_index (`self.Array Index`))
  (for (_array_element _array_index_2) (`self.ArrayBool`)
    (if (not _array_element)
      (set `self.Array Index` _array_index_2)
      (break)))
  (set `self.ItemLocation` (`SceneComponent.K2_GetComponentLocation` (`|GetArrayItem` (`self.ItemSockets`) _array_index)))
  (`KismetArrayLibrary.Array_Set` (`self.ArrayBool`) _array_index true))

(fn `UserConstructionScript`
  (`parent.UserConstructionScript`))